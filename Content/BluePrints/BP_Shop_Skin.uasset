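; Shop display actor that sells a player skin color to BP_Bot in exchange for collected trinkets.
; The preview mesh spins via LeftSpin while a looping timer flip-flops it between Antbot walk and run animations.
; Entering the trigger buys the skin once if affordable, deducting trinkets, applying it and updating the price text.
; Later overlaps reapply the purchased skin for free, while insufficient trinkets only print a message.
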(event OnComponentBeginOverlap(TriggerVolumeBox)
  (params (OverlappedComponent :type Primitive%20Component%20Object%20Reference) (OtherActor :type Actor%20Object%20Reference) (OtherComp :type Primitive%20Component%20Object%20Reference) (OtherBodyIndex :type Integer) (bFromSweep :type Boolean) (SweepResult :type Hit%20Result%20Structure%20%28by%20ref%29))
  (if (== (Utilities|GetClass OtherActor) "/Game/Framework/BP_Bot.BP_Bot_C")
    (bind _asbp_bot (Utilities|Casting|CastToBP_Bot OtherActor))
    (Variables|Default|SetAs%20BP%20Bot _asbp_bot)
    (if (Variables|Default|GetPurchased?)
      (Default|SetSkin (Variables|Default|GetAs%20BP%20Bot) (Variables|Default|GetPlayerSkinColorNumber))
      (elif (<= (Variables|Default|GetPrice_NumTrinkets) (Variables|/Game/Framework/BP_Bot.BP_Bot_C|GetNumCollectedTrinkets (Variables|Default|GetAs%20BP%20Bot)))
        (Utilities|FlowControl|DoOnce false
          (:Completed
            (Variables|Default|SetPurchased? true)
            (Default|DecreaseTrinketCounter (Variables|Default|GetAs%20BP%20Bot) (Variables|Default|GetPrice_NumTrinkets))
            (Default|SetSkin (Variables|Default|GetAs%20BP%20Bot) (Variables|Default|GetPlayerSkinColorNumber))
            (Rendering|Components|TextRender|SetText (Variables|Default|GetPrice) (Utilities|Text|MakeLiteralText "Purchased!"))))
        (else
          (Development|PrintString "\"You have insufficent Trinkets\""))))))

(event Custom|swapAnim
  (bind _skeletalmesh (Variables|Default|GetSkeletalMesh))
  (bind _isa (Utilities|FlowControl|FlipFlop)
    (:A
      _)
    (:B
      _))
  (if _isa
    (Components|Animation|PlayAnimation _skeletalmesh "/Game/Character/A_Antbot_Run.A_Antbot_Run" true)
    (else
      (Components|Animation|PlayAnimation _skeletalmesh "/Game/Character/A_Antbot_Walk.A_Antbot_Walk" true))))

(event EventBeginPlay
  (Components|Movement|SetUpdatedComponent (Variables|Default|GetleftSpin) (Variables|Default|GetSkeletalMesh))
  (Utilities|Time|SetTimerbyFunctionName 0 "swapAnim" 3.0 true)
  (Rendering|Components|TextRender|SetText (Variables|Default|GetPrice) (Utilities|Text|MakeLiteralText (Utilities|Text|ToText(String) (Utilities|String|Append (Utilities|String|MakeLiteralString "Price: ") (Utilities|String|ToString(Integer) (Variables|Default|GetPrice_NumTrinkets)) " Trinkets"))))
  (if (Variables|Default|GetPurchased?)
    (Rendering|Components|TextRender|SetText (Variables|Default|GetPrice) (Utilities|Text|MakeLiteralText "Purchased!"))))

(event Collision|EventActorBeginOverlap
  (params (OtherActor :type Actor%20Object%20Reference)))

(fn ConstructionScript)