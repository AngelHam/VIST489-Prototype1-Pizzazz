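; Gate actor Blueprint that exposes OpenGate and CloseGate events, guarded by an IsOpenGate flag.
; Each event sets every direct child component of SharedRoot to a fixed relative location, far down to open and far up to close, instantly without animation.
; Only opening plays a 2D sound (Invalid_Action).
; Redundant calls just print an error.
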(event Custom|CloseGate
  (if (not (Variables|Default|GetIsOpenGate))
    (Development|PrintString "ERROR: cannot close an already closed gate")
    (else
      (for _array_element (Components|GetChildrenComponents (Variables|Default|GetSharedRoot) false)
        (Transformation|SetRelativeLocation _array_element "0.000000,0.000000,3000.000000" false false))
      (Variables|Default|SetIsOpenGate false))))

(event Custom|OpenGate
  (if (Variables|Default|GetIsOpenGate)
    (Development|PrintString "ERROR: cannot open an already opened gate")
    (else
      (for _array_element (Components|GetChildrenComponents (Variables|Default|GetSharedRoot) false)
        (Transformation|SetRelativeLocation _array_element "0.000000,0.000000,-3000.000000" false false))
      (Variables|Default|SetIsOpenGate true)
      (Audio|PlaySound2D "/Engine/VREditor/Sounds/UI/Invalid_Action.Invalid_Action" 1.0 1.0 0.0 0 0))))

(event EventBeginPlay)

(event Collision|EventActorBeginOverlap
  (params (OtherActor :type Actor%20Object%20Reference)))

(event EventTick
  (params (DeltaSeconds :type Float%20%28single-precision%29)))

(fn ConstructionScript)