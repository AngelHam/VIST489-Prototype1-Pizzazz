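; Soul terminal actor that opens a text input screen when a BP_Bot enters its capsule.
; On BeginPlay it copies MySoulCode from the player controller and pre-creates the TextInputWidget.
; On overlap it swaps the bot's HUD for that widget, switches to UI-only input and shows the cursor.
; The end-overlap event is empty, and the logic to restore the HUD and game input is disconnected.
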(event OnComponentBeginOverlap(Capsule)
  (params (OverlappedComponent :type Primitive%20Component%20Object%20Reference) (OtherActor :type Actor%20Object%20Reference) (OtherComp :type Primitive%20Component%20Object%20Reference) (OtherBodyIndex :type Integer) (bFromSweep :type Boolean) (SweepResult :type Hit%20Result%20Structure%20%28by%20ref%29))
  (bind _returnvalue (Game|GetPlayerController 0))
  (bind _textinputwidget (Variables|Default|GetTextInputWidget))
  (if (== (Utilities|GetClass OtherActor) "/Game/Framework/BP_Bot.BP_Bot_C")
    (bind _asbp_bot (Utilities|Casting|CastToBP_Bot OtherActor))
    (Widget|RemovefromParent (Variables|/Game/Framework/BP_Bot.BP_Bot_C|GetHUD _asbp_bot))
    (UserInterface|Viewport|AddtoViewport _textinputwidget 0)
    (Input|SetInputModeUIOnly _returnvalue _textinputwidget "LockAlways" true)
    (Widget|SetFocus _textinputwidget)
    (Variables|/Script/Engine.PlayerController|SetbShowMouseCursor _returnvalue true)))

(event OnComponentEndOverlap(Capsule)
  (params (OverlappedComponent :type Primitive%20Component%20Object%20Reference) (OtherActor :type Actor%20Object%20Reference) (OtherComp :type Primitive%20Component%20Object%20Reference) (OtherBodyIndex :type Integer))
  ;[1 1 1] dep
)

(event EventBeginPlay
  (bind _returnvalue (Game|GetPlayerController 0))
  (bind _asbp_player_controller (Utilities|Casting|CastToBP_PlayerController _returnvalue))
  (Variables|Default|SetMy%20Soul%20Code (Variables|/Game/Framework/BP_PlayerController.BP_PlayerController_C|GetMySoulCode _asbp_player_controller))
  (bind _returnvalue_2 (UserInterface|CreateWidget "/Game/Framework/TextInputWidget.TextInputWidget_C" _returnvalue))
  (Variables|Default|SetTextInputWidget _returnvalue_2))

(event Collision|EventActorBeginOverlap
  (params (OtherActor :type Actor%20Object%20Reference)))

(event EventTick
  (params (DeltaSeconds :type Float%20%28single-precision%29)))

(fn ConstructionScript)