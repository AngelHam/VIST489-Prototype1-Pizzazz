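; Level-end goal actor that sends the player to the next level when a BP_Bot overlaps its collision component.
; The overlap plays a teleport effect, waits two seconds, then saves the player into MyNewGameInstance and calls NextLevel.
; The effect attaches a spawn particle system to the bot's mesh and loops a delayed sound with rising pitch.
; Older checkpoint-teleport logic remains disconnected.
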(event OnComponentBeginOverlap(FINISHGOAL_CollisionComp)
  (params (OverlappedComponent :type Primitive%20Component%20Object%20Reference) (OtherActor :type Actor%20Object%20Reference) (OtherComp :type Primitive%20Component%20Object%20Reference) (OtherBodyIndex :type Integer) (bFromSweep :type Boolean) (SweepResult :type Hit%20Result%20Structure%20%28by%20ref%29))
  (if (== (Utilities|GetClass OtherActor) "/Game/Framework/BP_Bot.BP_Bot_C")
    (CallFunction|PLayNoise+Effect)
    ;[1 1 1] Set the player's new checkpoint to the next map and teleport him there!
    (Utilities|FlowControl|Delay 2.0)
    (bind _asmy_new_game_instance (Utilities|Casting|CastToMyNewGameInstance (Game|GetGameInstance)))
    (Default|SavePLAYERIntoGameinstance _asmy_new_game_instance)
    (Default|NextLevel _asmy_new_game_instance)))

(event Custom|Play%20Noise%20+%20Effect
  ;[1 1 1] sound and visuals that play when you teleport
  (bind _returnvalue (Actor|GetActorOfClass "/Game/Framework/BP_Bot.BP_Bot_C"))
  (Niagara|SpawnSystemAttached "/Game/Assets/NIAGARA/PlayerSpawns.PlayerSpawns" (Variables|/Script/Engine.Character|GetMesh _returnvalue) "None" "0, 0, 0" "0, 0, 0" "SnapToTargetIncludingScale" false true "None" false)
  (Utilities|FlowControl|Delay 0.2 :!label _label)
  (if (<= (Variables|Default|GetintNoiseCount) 4)
    (Audio|PlaySound2D "/Game/Assets/death_01.death_01" 0.6 (+ (* (Math|Conversions|ToFloat(Integer) (Variables|Default|GetintNoiseCount)) 0.2) 1.0) 0.0 0 0)
    (bind _result (Math|Integer|IncrementInt (Variables|Default|GetintNoiseCount))
      (:%20%20
        (Variables|Default|SetintNoiseCount _result)
        (goto _label)))))

(event EventBeginPlay)

(event Collision|EventActorBeginOverlap
  (params (OtherActor :type Actor%20Object%20Reference)))

(event EventTick
  (params (DeltaSeconds :type Float%20%28single-precision%29)))

(fn ConstructionScript)