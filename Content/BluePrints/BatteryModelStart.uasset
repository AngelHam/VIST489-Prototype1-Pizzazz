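; Battery puzzle controller that runs a ball-and-lights puzzle and opens a linked gate when solved.
; An overlap moves PlayerBall to the starting battery; Tick rebinds ball and controller events and records triggered lights into SolutionAttempt.
; At puzzle end, a solution match can grant an extra jump, while the ball's failure event reloads whiteBox.
; On the editor plane, controller events freeze and hide BP_Bot, alternate two edit cameras, and restore it on exit.
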(event OnComponentBeginOverlap(EditorStart)
  (params (OverlappedComponent :type Primitive%20Component%20Object%20Reference) (OtherActor :type Actor%20Object%20Reference) (OtherComp :type Primitive%20Component%20Object%20Reference) (OtherBodyIndex :type Integer) (bFromSweep :type Boolean) (SweepResult :type Hit%20Result%20Structure%20%28by%20ref%29))
  ;[1 1 1] Check if player is on the plane that allows them to edit
  (if (== (Utilities|GetClass OtherActor) "/Game/Framework/BP_Bot.BP_Bot_C")
    (Variables|Default|SetPlayerHere true)))

(event OnComponentEndOverlap(EditorStart)
  (params (OverlappedComponent :type Primitive%20Component%20Object%20Reference) (OtherActor :type Actor%20Object%20Reference) (OtherComp :type Primitive%20Component%20Object%20Reference) (OtherBodyIndex :type Integer))
  ;[1 1 1] Check if player is on the plane that allows them to edit
  (if (== (Utilities|GetClass OtherActor) "/Game/Framework/BP_Bot.BP_Bot_C")
    (Variables|Default|SetPlayerHere false)))

(event OnComponentBeginOverlap(StartPuzzle)
  (params (OverlappedComponent :type Primitive%20Component%20Object%20Reference) (OtherActor :type Actor%20Object%20Reference) (OtherComp :type Primitive%20Component%20Object%20Reference) (OtherBodyIndex :type Integer) (bFromSweep :type Boolean) (SweepResult :type Hit%20Result%20Structure%20%28by%20ref%29))
  ;[1 1 1] Start Puzzle
  (Variables|Default|SetisPuzzleActive true)
  (if (== (Utilities|GetClass OtherActor) "/Game/Framework/BP_Bot.BP_Bot_C")
    (Utilities|FlowControl|DoOnce false
      (:Completed
        (Transformation|SetActorTransform (Variables|Default|GetPlayerBall) (Transformation|GetActorTransform (Variables|Default|GetStartingBattery)))
        (Game|Player|SetViewTargetwithBlend (Game|GetPlayerController 0) (Variables|Default|GetViewCamera) 0.0 "VTBlend_Linear" 0.0 false)
        (Variables|/Game/BluePrints/PlayerBall.PlayerBall_C|SetCurrentEndBattery (Variables|Default|GetPlayerBall) (Variables|Default|GetEndingBattery))
        (bind _asbp_player_controller (Utilities|Casting|CastToBP_PlayerController (Game|GetPlayerController 0)))
        (Default|TurnOn/OffEditClicks _asbp_player_controller false)))))

(event Custom|CameraExit
  ;[1 1 1] Exit the Editor
  (if (Variables|Default|GetPlayerHere)
    (bind _asbp_player_controller (Utilities|Casting|CastToBP_PlayerController (Game|GetPlayerController 0)))
    (Default|TurnOn/OffEditClicks _asbp_player_controller false)
    (if true
      (bind _returnvalue (Actor|GetActorOfClass "/Game/Framework/BP_Bot.BP_Bot_C"))
      (Transformation|SetActorTransform _returnvalue (Transformation|GetWorldTransform (Variables|Default|GetPlane)))
      (Variables|Default|SetEnterEditMode false)
      (Variables|/Script/Engine.CharacterMovementComponent|SetMaxWalkSpeed (Variables|/Script/Engine.Character|GetCharacterMovement _returnvalue) 1e+03)
      (Variables|/Script/Engine.CharacterMovementComponent|SetGravityScale (Variables|/Script/Engine.Character|GetCharacterMovement _returnvalue) 1.0)
      (Variables|/Script/Engine.Character|SetJumpMaxCount _returnvalue (Variables|/Game/Framework/BP_Bot.BP_Bot_C|GetCurrMaxJumpCount _returnvalue))
      (Rendering|SetActorHiddenInGame _returnvalue false)
      (Game|Player|SetViewTargetwithBlend (Game|GetPlayerController 0) (Variables|Default|GetPlayerCharacter) 1.5 "VTBlend_EaseInOut" 3.0 true)
      (Utilities|FlowControl|Delay 1.25))))

(event Custom|CameraStart
  (bind _playercharacter (Variables|Default|GetPlayerCharacter))
  (bind _charactermovement (Variables|/Script/Engine.Character|GetCharacterMovement _playercharacter))
  ;[1 1 1] Start Editor / Swap Cameras
  (if (Variables|Default|GetPlayerHere)
    (bind _asbp_player_controller (Utilities|Casting|CastToBP_PlayerController (Game|GetPlayerController 0)))
    (Default|TurnOn/OffEditClicks _asbp_player_controller true)
    (bind _returnvalue (Actor|GetActorOfClass "/Game/Framework/BP_Bot.BP_Bot_C"))
    (Variables|/Script/Engine.Character|SetJumpMaxCount _returnvalue 0)
    (Variables|/Script/Engine.MovementComponent|SetVelocity _charactermovement "0, 0, 0")
    (Variables|/Script/Engine.CharacterMovementComponent|SetMaxWalkSpeed _charactermovement 0.0)
    (Variables|/Script/Engine.CharacterMovementComponent|SetGravityScale _charactermovement 0.0)
    (Variables|Default|SetEnterEditMode true)
    (Rendering|SetActorHiddenInGame (Variables|Default|GetPlayerCharacter) true)
    (if (Variables|Default|GetCameraSwap)
      (Game|Player|SetViewTargetwithBlend (Game|GetPlayerController 0) (Variables|Default|GetEditor%201%20Camera) 1.5 "VTBlend_EaseInOut" 3.0 true)
      (Variables|Default|SetCameraSwap false)
      (Utilities|FlowControl|Delay 1.25)
      (else
        (Game|Player|SetViewTargetwithBlend (Game|GetPlayerController 0) (Variables|Default|GetEditor%202%20Camera) 1.5 "VTBlend_EaseInOut" 3.0 true)
        (Variables|Default|SetCameraSwap true)
        (Utilities|FlowControl|Delay 1.25)))))

(event Custom|ReachedEndCurrentPuzzle_Event
  ;[1 1 1] Check if matches solution, if true, send event dispatch to gate
  (if (Variables|Default|GetisPuzzleActive)
    (if (Utilities|Array|Identical (Variables|Default|GetSolutionAttempt) (Variables|/Game/BluePrints/Solution_BP.Solution_BP_C|GetSolution (Variables|Default|GetSolutionBoard)))
      (Development|PrintString "Level Complete, opening gate")
      (Audio|PlaySoundatLocation "/Game/Assets/lightPowered_Cue.lightPowered_Cue" "0, 0, 0" "0, 0, 0" 1.0 1.0 0.0 0 0 0 0)
      (Variables|/Script/Engine.CharacterMovementComponent|SetMaxWalkSpeed (Variables|/Script/Engine.Character|GetCharacterMovement (Game|GetPlayerCharacter 0)) 1e+03)
      (Variables|Default|SetPlayerHere true)
      (Variables|Default|SetisPuzzleActive false)
      ;;[1 1 1] If this is the right puzzle, allow double jump reward now :)
      (if (Variables|Default|GetDoubleJumpReward?)
        (bind _returnvalue (Actor|GetActorOfClass "/Game/Framework/BP_Bot.BP_Bot_C"))
        (bind _output_get (Variables|/Game/Framework/BP_Bot.BP_Bot_C|SetCurrMaxJumpCount _returnvalue (+ (Variables|/Game/Framework/BP_Bot.BP_Bot_C|GetCurrMaxJumpCount _returnvalue) 1)))
        (Development|PrintString (Utilities|String|ToString(Integer) _output_get))
        (Development|PrintString "CHARACTER PROGRESSION: DOUBLE JUMP")
        (bind _returnvalue_2 (Actor|GetActorOfClass "/Game/Framework/BP_Bot.BP_Bot_C"))
        (bind _result (Math|Integer|IncrementInt (Variables|/Game/Framework/BP_Bot.BP_Bot_C|GetPuzzleNum _returnvalue_2))
          (:%20%20
            (Variables|Default|SetPuzzleNumber _result))))
      (CallFunction|CameraExit)
      (Default|OpenGate (Variables|Default|GetGateToOpen)))))

(event Custom|FailedReachedEndCurrentPuzzle_Event
  ;[1 1 1] Failed puzzle, restart level at latest checkpoint
  (Development|PrintString "Failed restarting level")
  (Game|OpenLevel(byName) "whiteBox"))

(event EventBeginPlay
  ;[1 1 1] Set some object connections
  (bind _returnvalue (Actor|GetActorOfClass "/Game/BluePrints/PlayerBall.PlayerBall_C"))
  (Variables|Default|SetPlayerBall _returnvalue)
  (bind _returnvalue_2 (Actor|GetActorOfClass "/Game/Framework/BP_Bot.BP_Bot_C"))
  (Variables|Default|SetPlayerCharacter _returnvalue_2))

(event EventTick
  (params (DeltaSeconds :type Float%20%28single-precision%29))
  (bind _playerball (Variables|Default|GetPlayerBall))
  (bind _asbp_player_controller (Utilities|Casting|CastToBP_PlayerController (Game|GetPlayerController 0)))
  (EventDispatchers|BindEventtoEditorCameraSwap _asbp_player_controller (delegate Custom|CameraStart))
  (EventDispatchers|BindEventtoEditorCameraExit _asbp_player_controller (delegate Custom|CameraExit))
  (EventDispatchers|AssignReachedEndofCurrentPuzzle _playerball (delegate Custom|ReachedEndCurrentPuzzle_Event))
  (EventDispatchers|AssignFailedReachEndofCurrentPuzzle _playerball (delegate Custom|FailedReachedEndCurrentPuzzle_Event))
  (bind (_array_element _array_index) (Utilities|Array|ForEachLoopwithBreak (Variables|Default|GetLightArray))
    (:LoopBody
      ;[1 1 1] If in solution, update the menu UI and current solution attempt
      (Utilities|IsValid _array_element
        (:Is%20Valid
          (if (Variables|/Game/BluePrints/Light_And_Resistors.Light_And_Resistors_C|GetTriggered _array_element)
            (Utilities|Array|SetArrayElem (Variables|Default|GetSolutionAttempt) _array_index true)))))))

(fn ConstructionScript)