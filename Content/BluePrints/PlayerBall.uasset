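; PlayerBall is the ball that travels through circuit puzzles along splines owned by switches, wires, resistors and lights.
; Overlapping a piece selects its spline by whichever receiver is nearer.
; If active, MovePlayer drives it with a timeline whose play rate scales with spline length, selected speed and puzzle modifier.
; When movement finishes, proximity to the end battery reports reached or, after failure effects and a delay, failed to the current puzzle.
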(event Custom|Set%20Puzzle
  (params (Puzzle%20Object :type Battery%20Model%20Start%20Object%20Reference) (SpeedModifier :type Float%20%28double-precision%29))
  ;[1 1 1] Set Puzzle Object and its speed modifier to change ball speed
  (Variables|Default|SetPuzzlecurrent Puzzle%20Object)
  (Variables|Default|SetPuzzle%20Speed%20Modifier SpeedModifier))

(event Custom|TeleportToOutOfMap
  (bind _outofmap (Variables|Default|GetOutOfMap))
  (bind (_location _rotation) (Math|Transform|BreakTransform _outofmap))
  (Transformation|SetActorLocationAndRotation _location _rotation))

(event Custom|MovePlayer
  (params (Spline :type Spline%20Component%20Object%20Reference))
  (bind _currentendbattery (Variables|Default|GetCurrentEndBattery))
  (bind _defaultsceneroot (Variables|Default|GetDefaultSceneRoot))
  (bind _returnvalue (Transformation|GetWorldLocation _defaultsceneroot))
  (bind _rootcomponent (Variables|/Script/Engine.Actor|GetRootComponent _currentendbattery))
  (bind _returnvalue_2 (Transformation|GetWorldLocation _rootcomponent))
  (if (Variables|Default|Getactive%20player)
    (Development|PrintString "MovePlayer")
    (bind _output_get (Variables|Default|SetCurrentSpline Spline))
    (Components|Timeline|SetPlayRate (Variables|Default|GetMoveAlongLine) (/ 1.0 (/ (Spline|GetSplineLength _output_get) (* (* (Utilities|Array|Get(acopy) (Variables|Default|GetSpeed%20Values) (Variables|Default|GetSpeed%20Selector)) 0.5) (Variables|Default|GetPuzzle%20Speed%20Modifier)))))
    (Components|Timeline|SetNewTime (Variables|Default|GetMoveAlongLine) (Variables|Default|GetPlayerStartOffset))
    (bind _move (Timeline|MoveAlongLine Play)
      (:Update
        (Variables|Default|SetMove _move)
        (Transformation|SetActorLocationAndRotation (Spline|GetLocationatDistanceAlongSpline (Variables|Default|GetCurrentSpline) (Math|Float|Lerp 0.0 (Spline|GetSplineLength (Variables|Default|GetCurrentSpline)) (Variables|Default|GetMove)) "World") (Spline|GetRotationatDistanceAlongSpline (Variables|Default|GetCurrentSpline) (Math|Float|Lerp 0.0 (Spline|GetSplineLength (Variables|Default|GetCurrentSpline)) (Variables|Default|GetMove)) "World") true)
        (Variables|Default|SetballLocation (Transformation|GetWorldLocation (Variables|Default|GetSphere))))
      (:Finished
        ;[1 1 1] Win lose logic of the puzzles
        (Development|PrintString (Utilities|String|ToString(Vector) _returnvalue_2))
        (Development|PrintString (Utilities|String|ToString(Vector) _returnvalue))
        ;;[1 1 1] Did Playerball reach the end? True = Update UI Playerball Check
        (if (Utilities|Operators|EqualEqual _returnvalue_2 _returnvalue 1.5e+02)
          ;;[1 1 1] Did player ball hit all the lights correctly and get correct solution?
          (Default|ReachedEndCurrentPuzzleEvent (Variables|Default|GetPuzzlecurrent))
          (else
            (Audio|PlaySoundatLocation "/Game/Assets/death_04_Cue.death_04_Cue" "0, 0, 0" "0, 0, 0" 1.0 1.0 0.0 0 0 0 0)
            (Niagara|SpawnSystematLocation "/Game/Assets/NIAGARA/switchTurn.switchTurn" (Transformation|GetWorldLocation (Variables|Default|GetSphere)) "0, 0, 0" "3.000000,3.000000,3.000000")
            (Utilities|FlowControl|Delay 2.0)
            (Default|FailedReachedEndCurrentPuzzleEvent (Variables|Default|GetPuzzlecurrent))))))))

(event EventBeginPlay
  ;[1 1 1] Print SpeedValue at Start
  (Variables|Default|SetOutOfMap (Transformation|GetWorldTransform (Variables|Default|GetDefaultSceneRoot))))

(event Collision|EventActorBeginOverlap
  (params (OtherActor :type Actor%20Object%20Reference))
  (bind _sphere (Variables|Default|GetSphere))
  (bind _sphere_2 (Variables|Default|GetSphere))
  (bind _sphere_3 (Variables|Default|GetSphere))
  (bind _sphere_4 (Variables|Default|GetSphere))
  (bind _returnvalue (Transformation|GetWorldLocation _sphere))
  (bind _returnvalue_2 (Transformation|GetWorldLocation _sphere_2))
  (bind _returnvalue_3 (Transformation|GetWorldLocation _sphere_3))
  (bind _returnvalue_4 (Transformation|GetWorldLocation _sphere_4))
  ;[1 1 1] Triggers for Switch, Switch Straightaway, Wire to play MoveBall
  (Variables|Default|SetOther%20Actor OtherActor)
  ;;[1 0.9704 0.3487] When Ball touches Switch
  (if (Utilities|ClassIsChildOf (Utilities|GetClass OtherActor) "/Game/BluePrints/Switch.Switch_C")
    (bind _asswitch (Utilities|Casting|CastToSwitch (Variables|Default|GetOther%20Actor)))
    (bind _output_get (Variables|Default|SetCurrentSwitch _asswitch))
    (if (< (Math|Vector|VectorLength (- _returnvalue_3 (Transformation|GetWorldLocation (Variables|/Game/BluePrints/Switch.Switch_C|GetFrontReceiver _output_get)))) (Math|Vector|VectorLength (- _returnvalue_3 (Transformation|GetWorldLocation (Variables|/Game/BluePrints/Switch.Switch_C|GetBackReceiver _output_get)))))
      (CallFunction|MovePlayer (Variables|/Game/BluePrints/Switch.Switch_C|GetForward_BlueToYellow (Variables|Default|GetCurrentSwitch)))
      (else
        (CallFunction|MovePlayer (Variables|/Game/BluePrints/Switch.Switch_C|GetReverse_YellowToBlue (Variables|Default|GetCurrentSwitch)))))
    (else
      ;;[1 0.3061 0.07469] When Ball touches Switch Straightaway
      (if (Utilities|ClassIsChildOf (Utilities|GetClass OtherActor) "/Game/BluePrints/Switch-Straightaway.Switch-Straightaway_C")
        (bind _asswitch__straightaway (Utilities|Casting|CastToSwitch-Straightaway (Variables|Default|GetOther%20Actor)))
        (if (< (Math|Vector|VectorLength (- _returnvalue_2 (Transformation|GetWorldLocation (Variables|/Game/BluePrints/Switch-Straightaway.Switch-Straightaway_C|GetFrontReceiver _asswitch__straightaway)))) (Math|Vector|VectorLength (- _returnvalue_2 (Transformation|GetWorldLocation (Variables|/Game/BluePrints/Switch-Straightaway.Switch-Straightaway_C|GetBackReceiver _asswitch__straightaway)))))
          (CallFunction|MovePlayer (Variables|/Game/BluePrints/Switch-Straightaway.Switch-Straightaway_C|GetForward_BlueToYellow _asswitch__straightaway))
          (else
            (CallFunction|MovePlayer (Variables|/Game/BluePrints/Switch-Straightaway.Switch-Straightaway_C|GetReverse_YellowToBlue _asswitch__straightaway))))
        (else
          ;;[0.4929 0.3032 1] When Ball touches Wire
          (if (Utilities|ClassIsChildOf (Utilities|GetClass OtherActor) "/Game/BluePrints/Wire.Wire_C")
            (bind _aswire (Utilities|Casting|CastToWire (Variables|Default|GetOther%20Actor)))
            (bind _output_get_2 (Variables|Default|SetCurrent%20Wire _aswire))
            (if (< (Math|Vector|VectorLength (- _returnvalue_4 (Transformation|GetWorldLocation (Variables|/Game/BluePrints/Wire.Wire_C|GetFrontReceiver _output_get_2)))) (Math|Vector|VectorLength (- _returnvalue_4 (Transformation|GetWorldLocation (Variables|/Game/BluePrints/Wire.Wire_C|GetBackReceiver _output_get_2)))))
              (CallFunction|MovePlayer (Variables|/Game/BluePrints/Wire.Wire_C|GetForward_GreenToRed (Variables|Default|GetCurrent%20Wire)))
              (Audio|PlaySoundatLocation "/Game/Assets/speedPad_Cue.speedPad_Cue" "0, 0, 0" "0, 0, 0" 1.0 1.0 0.0 0 0 0 0)
              (else
                (CallFunction|MovePlayer (Variables|/Game/BluePrints/Wire.Wire_C|GetReverse_RedToGreen (Variables|Default|GetCurrent%20Wire)))
                (Audio|PlaySoundatLocation "/Game/Assets/speedPad_Cue.speedPad_Cue" "0, 0, 0" "0, 0, 0" 1.0 1.0 0.0 0 0 0 0)))
            (else
              ;;[1 0.2365 0.5505] When Ball touches Resistor and Lights
              (if (Utilities|ClassIsChildOf (Utilities|GetClass OtherActor) "/Game/BluePrints/Light_And_Resistors.Light_And_Resistors_C")
                (bind _aslight_and_resistors (Utilities|Casting|CastToLight_And_Resistors (Variables|Default|GetOther%20Actor)))
                (if (< (Math|Vector|VectorLength (- _returnvalue (Transformation|GetWorldLocation (Variables|/Game/BluePrints/Light_And_Resistors.Light_And_Resistors_C|GetFrontReceiver-GREEN _aslight_and_resistors)))) (Math|Vector|VectorLength (- _returnvalue (Transformation|GetWorldLocation (Variables|/Game/BluePrints/Light_And_Resistors.Light_And_Resistors_C|GetBackReceiver-RED _aslight_and_resistors)))))
                  (CallFunction|MovePlayer (Variables|/Game/BluePrints/Light_And_Resistors.Light_And_Resistors_C|GetSplineAlpha-GreenToRed _aslight_and_resistors))
                  (else
                    (CallFunction|MovePlayer (Variables|/Game/BluePrints/Light_And_Resistors.Light_And_Resistors_C|GetSplineBeta _aslight_and_resistors))))))))))))

(fn ConstructionScript)