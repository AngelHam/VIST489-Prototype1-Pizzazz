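; BP_Shop_EchoUpgrade is a shop pickup that sells the Echo upgrade to BP_Bot for trinkets.
; Its preview mesh spins, alternating Antbot run and walk animations on a looping timer, while another timer restarts a Niagara effect.
; When the bot enters the trigger box with enough trinkets, a one-time purchase deducts the price, unlocks Echo, updates the price text and plays a sound.
; Insufficient trinkets play a failure sound instead.
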(event OnComponentBeginOverlap(TriggerVolumeBox)
  (params (OverlappedComponent :type Primitive%20Component%20Object%20Reference) (OtherActor :type Actor%20Object%20Reference) (OtherComp :type Primitive%20Component%20Object%20Reference) (OtherBodyIndex :type Integer) (bFromSweep :type Boolean) (SweepResult :type Hit%20Result%20Structure%20%28by%20ref%29))
  (if (== (Utilities|GetClass OtherActor) "/Game/Framework/BP_Bot.BP_Bot_C")
    (bind _returnvalue (Actor|GetActorOfClass "/Game/Framework/BP_Bot.BP_Bot_C"))
    (Variables|Default|SetAs%20BP%20Bot_0 _returnvalue)
    (if (not (Variables|Default|GetPurchased?))
      (if (<= (Variables|Default|GetPrice_NumTrinkets) (Variables|/Game/Framework/BP_Bot.BP_Bot_C|GetNumCollectedTrinkets (Variables|Default|GetAs%20BP%20Bot_0)))
        (Utilities|FlowControl|DoOnce false
          (:Completed
            (Variables|Default|SetPurchased? true)
            (Default|DecreaseTrinketCounter (Variables|Default|GetAs%20BP%20Bot_0) (Variables|Default|GetPrice_NumTrinkets))
            (Default|UnlockEcho (Variables|Default|GetAs%20BP%20Bot_0))
            (Rendering|Components|TextRender|SetText (Variables|Default|GetPrice) (Utilities|Text|MakeLiteralText "Purchased!"))
            (Audio|SpawnSound2D "/Game/Assets/mouseHover_01_Cue1.mouseHover_01_Cue1" 1.0 1.0 0.0 0)))
        (else
          (Audio|SpawnSound2D "/Game/Assets/death6_Cue.death6_Cue" 1.0 1.0 0.0 0))))))

(event Custom|particle
  (Components|Activation|SetActive (Variables|Default|GetNiagara) true true))

(event Custom|swapAnim
  (bind _skeletalmesh (Variables|Default|GetSkeletalMesh))
  (bind _isa (Utilities|FlowControl|FlipFlop)
    (:A
      _)
    (:B
      _))
  (if _isa
    (Components|Animation|PlayAnimation _skeletalmesh "/Game/Character/A_Antbot_Run.A_Antbot_Run" true)
    (else
      (Components|Animation|PlayAnimation _skeletalmesh "/Game/Character/A_Antbot_Walk.A_Antbot_Walk" true))))

(event EventBeginPlay
  (Components|Movement|SetUpdatedComponent (Variables|Default|GetleftSpin) (Variables|Default|GetSkeletalMesh))
  (Utilities|Time|SetTimerbyFunctionName 0 "swapAnim" 3.0 true)
  (Utilities|Time|SetTimerbyFunctionName 0 "particle" 0.2 true)
  (Rendering|Components|TextRender|SetText (Variables|Default|GetPrice) (Utilities|Text|MakeLiteralText (Utilities|Text|ToText(String) (Utilities|String|Append (Utilities|String|MakeLiteralString "Price: ") (Utilities|String|ToString(Integer) (Variables|Default|GetPrice_NumTrinkets)) " Trinkets"))))
  (if (Variables|Default|GetPurchased?)
    (Rendering|Components|TextRender|SetText (Variables|Default|GetPrice) (Utilities|Text|MakeLiteralText "Purchased!"))))

(event Collision|EventActorBeginOverlap
  (params (OtherActor :type Actor%20Object%20Reference)))

(fn ConstructionScript)