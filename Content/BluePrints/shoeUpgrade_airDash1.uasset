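; Air dash shoe pickup that grants BP_Bot the ability to air dash.
; On BeginPlay it binds four CounterMovement components to their meshes and plays an aura sound.
; The first bot overlap, gated by DoOnce, plays pickup effects, hides the display shoes and aura, and stops the audio component.
; It then hides the bot's current shoes, attaches ShoeBP2 to both shoe sockets and sets CanAirDash.
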(event EventBeginPlay
  ;[1 1 1] LOOK AT ALL THIS CODE ANGEL MY DEV BRAIN IS ENLARGERNINAAANINGGGGGGG
  ;;[1 1 1] Make VFX and SFX play during level initialization
  (Components|Movement|SetUpdatedComponent (Variables|Default|GetcounterMovement) (Variables|Default|GetFloor1470_StaticMeshComponent0))
  (Components|Movement|SetUpdatedComponent (Variables|Default|GetcounterMovement2) (Variables|Default|GetFloor1471_StaticMeshComponent0))
  (Components|Movement|SetUpdatedComponent (Variables|Default|GetcounterMovement3) (Variables|Default|GetCylinder7_StaticMeshComponent0))
  (Components|Movement|SetUpdatedComponent (Variables|Default|GetcounterMovement4) (Variables|Default|GetStaticMesh))
  (Audio|PlaySoundatLocation "/Game/Assets/respawnAura_Cue.respawnAura_Cue" (Transformation|GetActorLocation) "0, 0, 0" 1.0 1.0 0.0 0 0 0 0))

(event Collision|EventActorBeginOverlap
  (params (OtherActor :type Actor%20Object%20Reference))
  (bind _returnvalue (Transformation|GetActorLocation))
  ;[1 1 1] LOOK AT ALL THIS CODE ANGEL MY DEV BRAIN IS ENLARGERNINAAANINGGGGGGG
  ;;[1 1 1] player recieves double jump, vfx and sfx end
  (if (== (Utilities|GetClass OtherActor) "/Game/Framework/BP_Bot.BP_Bot_C")
    (bind _asbp_bot (Utilities|Casting|CastToBP_Bot OtherActor))
    (Variables|Default|SetPlayer%20Character _asbp_bot)
    (Utilities|FlowControl|DoOnce false
      (:Completed
        (Audio|PlaySoundatLocation "/Game/Assets/trinketGet2_Cue.trinketGet2_Cue" _returnvalue "0, 0, 0" 1.0 1.0 0.0 0 0 0 0)
        (Niagara|SpawnSystematLocation "/Game/Assets/NIAGARA/trinketGet.trinketGet" _returnvalue)
        (Rendering|SetVisibility (Variables|Default|GetbotShoe_airDash_01) false false)
        (Audio|Components|Audio|Stop (Variables|Default|GetrespawnAura_Cue4_AudioComponent0))
        (Actor|GetActorOfClass "/Game/Framework/BP_Bot.BP_Bot_C")
        ;;[1 1 1] Spawn Shoes on Player Skeleton
        (for _array_element (Components|GetChildrenComponents (Variables|/Script/Engine.Character|GetMesh (Variables|Default|GetPlayer%20Character)) true)
          (Default|HideShoes+MeshDescendents (Variables|Default|GetPlayer%20Character)))
        (bind _returnvalue_2 (Game|SpawnActorfromClass "/Game/BluePrints/shoeBP2.shoeBP2_C" (Transformation|GetSocketTransform (Variables|/Script/Engine.Character|GetMesh (Variables|Default|GetPlayer%20Character)) "shoe_lSocket" "RTS_World") "Undefined" 0 0))
        (Transformation|AttachComponentToComponent _returnvalue_2 (Variables|/Script/Engine.Character|GetMesh (Variables|Default|GetPlayer%20Character)) "shoe_lSocket" "SnapToTarget" "SnapToTarget" "SnapToTarget" true)
        (bind _returnvalue_3 (Game|SpawnActorfromClass "/Game/BluePrints/shoeBP2.shoeBP2_C" (Transformation|GetSocketTransform (Variables|/Script/Engine.Character|GetMesh (Variables|Default|GetPlayer%20Character)) "shoe_rSocket" "RTS_World") "Undefined" 0 0))
        (Transformation|AttachComponentToComponent _returnvalue_3 (Variables|/Script/Engine.Character|GetMesh (Variables|Default|GetPlayer%20Character)) "shoe_rSocket" "SnapToTarget" "SnapToTarget" "SnapToTarget" true)
        ;;[1 1 1] Enable More Jumps
        (Variables|/Game/Framework/BP_Bot.BP_Bot_C|SetCanAirDash (Variables|Default|GetPlayer%20Character) true)))))

(event EventTick
  (params (DeltaSeconds :type Float%20%28single-precision%29))
  ;[1 1 1] LOOK AT ALL THIS CODE ANGEL MY DEV BRAIN IS ENLARGERNINAAANINGGGGGGG
)

(fn ConstructionScript)