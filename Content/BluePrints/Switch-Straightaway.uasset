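; Straightaway piece of a switch that turns in alternating steps each time its Rotate event is called.
; Rotate plays a switch sound and spawns a turn effect above the Sphere component, then branches on the 2ndCall flag.
; The first call adds 90 degrees to the current rotation.
; The second resets to a fixed 45-degree rotation and tells the parent Switch actor to run ToggleVisibilityReverse.
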(event Custom|Rotate
  (bind _returnvalue (Transformation|GetActorTransform))
  (bind _returnvalue_2 (Transformation|GetActorTransform))
  (bind _sphere (Variables|Default|GetSphere))
  (bind _returnvalue_3 (Transformation|GetWorldLocation _sphere))
  (bind (_location _rotation _scale) (Math|Transform|BreakTransform _returnvalue_2))
  (bind (_location_2 _rotation_2 _scale_2) (Math|Transform|BreakTransform _returnvalue))
  (bind _returnvalue_4 (+ _returnvalue_3 "0.000000,0.000000,300.000000"))
  (Audio|PlaySoundatLocation "/Game/Assets/switchSound_Cue.switchSound_Cue" _returnvalue_4 "0, 0, 0" 1.0 1.0 0.0 0 0 0 0)
  (Niagara|SpawnSystematLocation "/Game/Assets/NIAGARA/switchTurn.switchTurn" _returnvalue_4)
  (if (Variables|Default|Get2ndCall)
    (Transformation|SetActorTransform (Math|Transform|MakeTransform _location_2 "0.000000,45.000000,0.000000" _scale_2))
    (bind _asswitch (Utilities|Casting|CastToSwitch (Actor|GetParentActor)))
    (Default|ToggleVisibilityReverse _asswitch)
    (Variables|Default|Set2ndCall false)
    (else
      (Transformation|SetActorTransform (Math|Transform|MakeTransform _location (Math|Rotator|CombineRotators _rotation "0.000000,90.000000,0.000000") _scale))
      (Variables|Default|Set2ndCall true))))

(event EventBeginPlay)

(event Collision|EventActorBeginOverlap
  (params (OtherActor :type Actor%20Object%20Reference)))

(event EventTick
  (params (DeltaSeconds :type Float%20%28single-precision%29)))

(fn ConstructionScript)