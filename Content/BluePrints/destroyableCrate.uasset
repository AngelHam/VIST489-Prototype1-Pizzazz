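; Destructible crate actor that breaks when its punched event fires.
; Punching plays a small camera shake at the player camera, plus a Niagara effect and sound at the box's location.
; AddForce spawns an FS_MasterField actor there, an attempt at fracture destruction.
; The crate then removes itself from its ChildOfBoxSpawner's list, if that reference is valid, and destroys itself.
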(event Custom|punched
  (bind _blankbox (Variables|Default|GetblankBox))
  (bind _childofboxspawner_ (Variables|Default|GetChildOfBoxSpawner?))
  (bind _returnvalue (Transformation|GetWorldLocation _blankbox))
  (Camera|PlayWorldCameraShake "/Game/BluePrints/cameraShake_Small.cameraShake_Small_C" (Transformation|GetActorLocation (Game|GetPlayerCameraManager 0)) 0.0 5e+02)
  (Niagara|SpawnSystematLocation "/Game/Assets/NIAGARA/switchTurn.switchTurn" (Transformation|GetWorldLocation (Variables|Default|GetblankBox)))
  (Audio|PlaySoundatLocation "/Game/Assets/death_05_Cue.death_05_Cue" _returnvalue "0, 0, 0" 1.0 1.0 0.0 0 0 0 0)
  ;[1 1 1] Me and my dumb ass trying to get Fracture destruction to work
  (CallFunction|AddForce (Math|Conversions|ToTransform(Vector) _returnvalue))
  ;[1 1 1] Destroy the box, if its from a spawner, remove it from its list of references
  (if (Utilities|IsValid _childofboxspawner_)
    (Default|RemoveBoxfromList _childofboxspawner_ self))
  (Actor|DestroyActor))

(event Custom|Add%20Force
  (params (SpawnTransform :type Transform))
  ;[1 1 1] Me and my dumb ass trying to get Fracture destruction to work
  (Game|SpawnActorfromClass "/Engine/EditorResources/FieldNodes/FS_MasterField.FS_MasterField_C" SpawnTransform "Undefined" 0 0))

(event EventBeginPlay)

(event Collision|EventActorBeginOverlap
  (params (OtherActor :type Actor%20Object%20Reference)))

(event EventTick
  (params (DeltaSeconds :type Float%20%28single-precision%29)))

(fn ConstructionScript)