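; Puzzle circuit piece with a shielded star light and two resistors that the PlayerBall passes through.
; Each resistor cycles through four power levels with matching symbols, can toggle visibility, and writes its level to the ball's SpeedSelector on overlap.
; ForceFieldColor sets the shield material at BeginPlay.
; Light overlap fires the LightTriggered dispatcher, then lights the star and swaps the shield material if SpeedSelector matches ForceFieldColor, otherwise plays a fail sound.
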(event OnComponentBeginOverlap(Resistor2-RED)
  (params (OverlappedComponent :type Primitive%20Component%20Object%20Reference) (OtherActor :type Actor%20Object%20Reference) (OtherComp :type Primitive%20Component%20Object%20Reference) (OtherBodyIndex :type Integer) (bFromSweep :type Boolean) (SweepResult :type Hit%20Result%20Structure%20%28by%20ref%29))
  (if (Utilities|ClassIsChildOf (Utilities|GetClass OtherActor) "/Game/BluePrints/PlayerBall.PlayerBall_C")
    (bind _asplayer_ball (Utilities|Casting|CastToPlayerBall OtherActor))
    (Variables|/Game/BluePrints/PlayerBall.PlayerBall_C|SetSpeed%20Selector _asplayer_ball (Variables|Default|GetRes2Index-RED))))

(event OnComponentBeginOverlap(Resistor1-GREEN)
  (params (OverlappedComponent :type Primitive%20Component%20Object%20Reference) (OtherActor :type Actor%20Object%20Reference) (OtherComp :type Primitive%20Component%20Object%20Reference) (OtherBodyIndex :type Integer) (bFromSweep :type Boolean) (SweepResult :type Hit%20Result%20Structure%20%28by%20ref%29))
  (if (Utilities|ClassIsChildOf (Utilities|GetClass OtherActor) "/Game/BluePrints/PlayerBall.PlayerBall_C")
    (bind _asplayer_ball (Utilities|Casting|CastToPlayerBall OtherActor))
    (Variables|/Game/BluePrints/PlayerBall.PlayerBall_C|SetSpeed%20Selector _asplayer_ball (Variables|Default|GetRes1Index-GREEN))))

(event OnComponentBeginOverlap(Light)
  (params (OverlappedComponent :type Primitive%20Component%20Object%20Reference) (OtherActor :type Actor%20Object%20Reference) (OtherComp :type Primitive%20Component%20Object%20Reference) (OtherBodyIndex :type Integer) (bFromSweep :type Boolean) (SweepResult :type Hit%20Result%20Structure%20%28by%20ref%29))
  (bind _forcefieldcolor (Variables|Default|GetforceFieldColor))
  (if (Utilities|ClassIsChildOf (Utilities|GetClass OtherActor) "/Game/BluePrints/PlayerBall.PlayerBall_C")
    ;[1 1 1] Send a Event Dispatch to BatteryModelStart to tell that this light has been triggered
    (Variables|Default|SetTriggered true)
    (Default|CallLightTriggered)
    (bind _asplayer_ball (Utilities|Casting|CastToPlayerBall OtherActor))
    (Development|PrintString (Utilities|String|ToString(Integer) (Variables|/Game/BluePrints/PlayerBall.PlayerBall_C|GetSpeed%20Selector _asplayer_ball)))
    (Development|PrintString (Utilities|String|ToString(Integer) _forcefieldcolor))
    (if (== (Variables|/Game/BluePrints/PlayerBall.PlayerBall_C|GetSpeed%20Selector _asplayer_ball) _forcefieldcolor)
      (Audio|PlaySoundatLocation "/Game/Assets/lightPowered_Cue.lightPowered_Cue" "0, 0, 0" "0, 0, 0" 1.0 1.0 0.0 0 0 0 0)
      (Rendering|Material|SetMaterial (Variables|Default|Getstar) 0 "/Game/Assets/SCon_Mats/LitStar_Yellow2.LitStar_Yellow2")
      (Rendering|Material|SetMaterial (Variables|Default|Getshield) 0 "/Engine/Functions/Engine_MaterialFunctions02/ExampleContent/3dParticleOpacity_Mat.3dParticleOpacity_Mat")
      (else
        (Audio|PlaySoundatLocation "/Game/Assets/lightFail.lightFail" "0, 0, 0" "0, 0, 0" 1.0 1.0 0.0 0 0 0 0)))))

(event Custom|Toggle%20Existance%20Resistor2
  ;[1 1 1] For User/Player to toggle the existance of the resistor in "Edit" Mode, probably with left click
  (Rendering|ToggleVisibility (Variables|Default|GetResistor2-RED) true))

(event Custom|Toggle%20Existance%20Resistor1
  ;[1 1 1] For User/Player to toggle the existance of the resistor in "Edit" Mode, probably with left click
  (Rendering|ToggleVisibility (Variables|Default|GetResistor1-GREEN) true))

(event Custom|Cycle%20Through%20Resistor1%20Power
  ;[1 1 1] Cycle through 1,2,3 4 index selections for Resistor 1 and 2 (0 is reserved for 0 speed)
  (if (> (Variables|Default|GetRes1Index-GREEN) 3)
    (Variables|Default|SetRes1Index-GREEN 1)
    (else
      (Variables|Default|SetRes1Index-GREEN (+ 1 (Variables|Default|GetRes1Index-GREEN)))))
  (Audio|PlaySoundatLocation "/Game/Assets/mouseHover_01_Cue.mouseHover_01_Cue" "0, 0, 0" "0, 0, 0" 1.0 1.0 0.0 0 0 0 0)
  (Niagara|SpawnSystematLocation "/Game/Assets/NIAGARA/switchTurn.switchTurn" (Transformation|GetWorldLocation (Variables|Default|GetResistor1-GREEN)))
  (switch int (Variables|Default|GetRes1Index-GREEN)
    (:Default
      (Development|SetHiddeninGame (Variables|Default|Getresistance_Symbol_1_Entry) true false :!label _label)
      (Development|SetHiddeninGame (Variables|Default|Getresistance_Symbol_2_Entry) true false)
      (Development|SetHiddeninGame (Variables|Default|Getresistance_Symbol_3_Entry) true false))
    (:1
      (goto _label))
    (:2
      (Development|SetHiddeninGame (Variables|Default|Getresistance_Symbol_1_Entry) false false)
      (Development|SetHiddeninGame (Variables|Default|Getresistance_Symbol_2_Entry) true false)
      (Development|SetHiddeninGame (Variables|Default|Getresistance_Symbol_3_Entry) true false))
    (:3
      (Development|SetHiddeninGame (Variables|Default|Getresistance_Symbol_1_Entry) true false)
      (Development|SetHiddeninGame (Variables|Default|Getresistance_Symbol_2_Entry) false false)
      (Development|SetHiddeninGame (Variables|Default|Getresistance_Symbol_3_Entry) true false))
    (:4
      (Development|SetHiddeninGame (Variables|Default|Getresistance_Symbol_1_Entry) true false)
      (Development|SetHiddeninGame (Variables|Default|Getresistance_Symbol_2_Entry) true false)
      (Development|SetHiddeninGame (Variables|Default|Getresistance_Symbol_3_Entry) false false))))

(event Custom|Cycle%20Through%20Resistor2%20Power
  ;[1 1 1] Cycle through 1,2,3 4 index selections for Resistor 1 and 2 (0 is reserved for 0 speed)
  (if (> (Variables|Default|GetRes2Index-RED) 3)
    (Variables|Default|SetRes2Index-RED 1)
    (else
      (Variables|Default|SetRes2Index-RED (+ 1 (Variables|Default|GetRes2Index-RED)))))
  (Audio|PlaySoundatLocation "/Game/Assets/mouseHover_01_Cue.mouseHover_01_Cue" "0, 0, 0" "0, 0, 0" 1.0 1.0 0.0 0 0 0 0)
  (Niagara|SpawnSystematLocation "/Game/Assets/NIAGARA/switchTurn.switchTurn" (Transformation|GetWorldLocation (Variables|Default|GetResistor2-RED)))
  (switch int (Variables|Default|GetRes2Index-RED)
    (:1
      (Development|SetHiddeninGame (Variables|Default|Getresistance_Symbol_1_Entry1) true false)
      (Development|SetHiddeninGame (Variables|Default|Getresistance_Symbol_2_Entry1) true false)
      (Development|SetHiddeninGame (Variables|Default|Getresistance_Symbol_3_Entry1) true false))
    (:2
      (Development|SetHiddeninGame (Variables|Default|Getresistance_Symbol_1_Entry1) false false)
      (Development|SetHiddeninGame (Variables|Default|Getresistance_Symbol_2_Entry1) true false)
      (Development|SetHiddeninGame (Variables|Default|Getresistance_Symbol_3_Entry1) true false))
    (:3
      (Development|SetHiddeninGame (Variables|Default|Getresistance_Symbol_1_Entry1) true false)
      (Development|SetHiddeninGame (Variables|Default|Getresistance_Symbol_2_Entry1) false false)
      (Development|SetHiddeninGame (Variables|Default|Getresistance_Symbol_3_Entry1) true false))
    (:4
      (Development|SetHiddeninGame (Variables|Default|Getresistance_Symbol_1_Entry1) true false)
      (Development|SetHiddeninGame (Variables|Default|Getresistance_Symbol_2_Entry1) true false)
      (Development|SetHiddeninGame (Variables|Default|Getresistance_Symbol_3_Entry1) false false))))

(event EventBeginPlay
  (bind _shield (Variables|Default|Getshield))
  ;[1 1 1] Begin Play set the correct material of force fields to the star shields
  (switch int (Variables|Default|GetforceFieldColor)
    (:1
      (Rendering|Material|SetMaterial _shield 0 "/Engine/Functions/Engine_MaterialFunctions02/ExampleContent/3dParticleOpacity_Mat.3dParticleOpacity_Mat"))
    (:2
      (Rendering|Material|SetMaterial _shield 0 "/Engine/VREditor/TransformGizmo/Main.Main"))
    (:3
      (Rendering|Material|SetMaterial _shield 0 "/Engine/VREditor/TransformGizmo/main_yellow.main_yellow"))
    (:4
      (Rendering|Material|SetMaterial _shield 0 "/Engine/VREditor/TransformGizmo/main_red.main_red"))))

(fn ConstructionScript)