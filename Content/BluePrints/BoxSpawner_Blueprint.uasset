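; Box spawner actor that creates destroyable crates when the player pawn steps on its overlap trigger.
; The overlap spawns a DestroyableCrate at the SpawnPoint with a set scale, up to an allowed maximum, and prints a message otherwise.
; Each crate is tracked in an array and counter and given a reference back to the spawner, with RemoveBoxFromList available to unregister it and free a slot.
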(event OnComponentBeginOverlap(StepOnToSpawn)
  (params (OverlappedComponent :type Primitive%20Component%20Object%20Reference) (OtherActor :type Actor%20Object%20Reference) (OtherComp :type Primitive%20Component%20Object%20Reference) (OtherBodyIndex :type Integer) (bFromSweep :type Boolean) (SweepResult :type Hit%20Result%20Structure%20%28by%20ref%29))
  (if (== OtherActor (Game|Player|GetPlayerPawn 0))
    (CallFunction|SpawnDestroyableCrate)
    (else
      (Development|PrintString "Invalid Target Overlap"))))

(event Custom|Spawn%20DestroyableCrate
  (bind _spawnpoint (Variables|Default|GetspawnPoint))
  (if (< (Variables|Default|GetNumCratesCurrentlyExist) (Variables|Default|GetNumAllowedSpawnCrates))
    (bind _returnvalue (Game|SpawnActorfromClass "/Game/BluePrints/destroyableCrate.destroyableCrate_C" (Math|Transform|MakeTransform (Transformation|GetWorldLocation _spawnpoint) (Transformation|GetWorldRotation _spawnpoint) (Variables|Default|GetScaleOfBox)) "Undefined" 0 0))
    (Utilities|Array|Add (Variables|Default|GetCrates) _returnvalue)
    (Variables|/Game/BluePrints/destroyableCrate.destroyableCrate_C|SetChildOfBoxSpawner? _returnvalue self)
    (bind _result (Math|Integer|IncrementInt (Variables|Default|GetNumCratesCurrentlyExist))
      (:%20%20
        (Variables|Default|SetNumCratesCurrentlyExist _result)))
    (else
      (Development|PrintString "Reached Max Number of Crates"))))

(event Custom|RemoveBoxFromList
  (params (Crate :type Destroyable%20Crate%20Object%20Reference))
  (for _array_element (Variables|Default|GetCrates)
    (if (== _array_element Crate)
      (Utilities|Array|RemoveItem (Variables|Default|GetCrates) Crate)
      (bind _result (Math|Integer|DecrementInt (Variables|Default|GetNumCratesCurrentlyExist))
        (:%20%20
          (Variables|Default|SetNumCratesCurrentlyExist _result))))))

(event EventBeginPlay)

(event Collision|EventActorBeginOverlap
  (params (OtherActor :type Actor%20Object%20Reference)))

(event EventTick
  (params (DeltaSeconds :type Float%20%28single-precision%29)))

(fn ConstructionScript)