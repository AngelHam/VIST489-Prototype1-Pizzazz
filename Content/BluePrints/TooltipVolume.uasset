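; TooltipVolume is a trigger volume that shows a configurable tooltip as player dialogue on a BP_Bot's HUD when that bot enters it.
; On overlap it sets the speech delay and "player" headshot, then starts the dialogue text.
; A Delay loop polls the HUD's character count until the text finishes, then clears it after a pause.
; A DoOnce blocks retriggering until a further reset delay elapses.
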(event OnComponentBeginOverlap(CollisionComponent)
  (params (OverlappedComponent :type Primitive%20Component%20Object%20Reference) (OtherActor :type Actor%20Object%20Reference) (OtherComp :type Primitive%20Component%20Object%20Reference) (OtherBodyIndex :type Integer) (bFromSweep :type Boolean) (SweepResult :type Hit%20Result%20Structure%20%28by%20ref%29))
  (bind _tooltip (Variables|Default|GetToolTip))
  (if (== (Utilities|GetClass OtherActor) "/Game/Framework/BP_Bot.BP_Bot_C")
    (Utilities|FlowControl|DoOnce false :!label _label
      (:Completed
        (bind _asbp_bot (Utilities|Casting|CastToBP_Bot OtherActor))
        (Variables|/Game/Widgets/PlayerHUDTemp.PlayerHUDTemp_C|Setdelayspeech (Variables|/Game/Framework/BP_Bot.BP_Bot_C|GetHUD _asbp_bot) (Variables|Default|GetDelaySpeech))
        (Default|SetHeadshot (Variables|/Game/Framework/BP_Bot.BP_Bot_C|GetHUD _asbp_bot) "player")
        (Default|UpdateDialogue (Variables|/Game/Framework/BP_Bot.BP_Bot_C|GetHUD _asbp_bot) _tooltip)
        (Utilities|FlowControl|Delay 0.2 :!label _label_2)
        (if (> (Variables|/Game/Widgets/PlayerHUDTemp.PlayerHUDTemp_C|GetCharCount (Variables|/Game/Framework/BP_Bot.BP_Bot_C|GetHUD _asbp_bot)) (Utilities|String|Len _tooltip))
          (Utilities|FlowControl|Delay (Variables|Default|GetDelayBeforeDisappear))
          (Default|ClearTextDialogue (Variables|/Game/Framework/BP_Bot.BP_Bot_C|GetHUD _asbp_bot))
          (Utilities|FlowControl|Delay (Variables|Default|GetResetMessageTime))
          (goto _label Reset)
          (else
            (goto _label_2)))))))

(event EventBeginPlay)

(event Collision|EventActorBeginOverlap
  (params (OtherActor :type Actor%20Object%20Reference)))

(event EventTick
  (params (DeltaSeconds :type Float%20%28single-precision%29)))

(fn ConstructionScript)