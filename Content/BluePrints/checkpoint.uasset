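; Checkpoint actor that saves the player's respawn point when a BP_Bot enters its trigger.
; The overlap passes the SpawnPoint transform to BP_PlayerController and plays a checkpoint sound there, on every qualifying entry.
; BeginPlay points the RightSpin and LeftSpin movement components at two meshes each in succession, so only the last assignments, Cube2 and Cube4, remain their updated components.
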(event OnComponentBeginOverlap(CheckpointTrigger)
  (params (OverlappedComponent :type Primitive%20Component%20Object%20Reference) (OtherActor :type Actor%20Object%20Reference) (OtherComp :type Primitive%20Component%20Object%20Reference) (OtherBodyIndex :type Integer) (bFromSweep :type Boolean) (SweepResult :type Hit%20Result%20Structure%20%28by%20ref%29))
  (bind _spawnpoint (Variables|Default|GetSpawnPoint))
  (bind _returnvalue (Transformation|GetWorldTransform _spawnpoint))
  (if (== (Utilities|GetClass OtherActor) "/Game/Framework/BP_Bot.BP_Bot_C")
    (bind _asbp_player_controller (Utilities|Casting|CastToBP_PlayerController (Game|GetPlayerController 0)))
    (Default|SetCheckpointSpawn _asbp_player_controller _returnvalue)
    (Audio|SpawnSoundatLocation "/Game/Assets/CheckPointNoise_Cue.CheckPointNoise_Cue" (.Location (Math|Transform|BreakTransform _returnvalue)) "0, 0, 0" 1.0 1.0 0.0 0 0)))

(event EventBeginPlay
  (Components|Movement|SetUpdatedComponent (Variables|Default|GetrightSpin) (Variables|Default|GetStaticBase1))
  (Components|Movement|SetUpdatedComponent (Variables|Default|GetrightSpin) (Variables|Default|GetCube2))
  (Components|Movement|SetUpdatedComponent (Variables|Default|GetleftSpin) (Variables|Default|GetStaticBase2))
  (Components|Movement|SetUpdatedComponent (Variables|Default|GetleftSpin) (Variables|Default|GetCube4)))

(event Collision|EventActorBeginOverlap
  (params (OtherActor :type Actor%20Object%20Reference)))

(event EventTick
  (params (DeltaSeconds :type Float%20%28single-precision%29)))

(fn ConstructionScript)