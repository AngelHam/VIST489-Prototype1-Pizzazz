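; Player controller that moves the pawn and lets the player click circuit pieces to change them.
; Move Forward/Right axes add movement input from a rotator that carries control yaw in its roll slot.
; ToggleInput sets a flag that Tick consumes once, tracing under the cursor on Visibility.
; Hit Switch or SwitchStraightaway actors rotate; Light_And_Resistors cycles the power of whichever resistor component matches the hit by name.
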(event EventTick
  (params (DeltaSeconds :type Float%20%28single-precision%29))
  (bind _hitresult (Game|Player|GetHitResultUnderCursorbyChannel "TraceTypeQuery1" true))
  (bind (_bblockinghit _binitialoverlap _time _distance _location _impactpoint _normal _impactnormal _physmat _hitactor _hitcomponent) (Collision|BreakHitResult _hitresult))
  (bind _returnvalue (Utilities|GetClass _hitactor))
  ;[1 1 1] SHOULD BE FOR EDITING WITH LEFT CLICK
  (if (Variables|Default|GetLeftClick)
    (Variables|Default|SetLeftClick false)
    (Variables|Default|SetHit%20Component _hitcomponent)
    (Variables|Default|SetLeftClick%20Hit%20Actor _hitactor)
    (if (Utilities|ClassIsChildOf _returnvalue "/Game/Circuit/Switch.Switch_C")
      (bind _asswitch (Utilities|Casting|CastToSwitch (Variables|Default|GetLeftClick%20Hit%20Actor)))
      (Default|Rotate _asswitch)
      (elif (Utilities|ClassIsChildOf _returnvalue "/Game/Circuit/Switch-Straightaway.Switch-Straightaway_C")
        (bind _asswitch__straightaway (Utilities|Casting|CastToSwitch-Straightaway (Variables|Default|GetLeftClick%20Hit%20Actor)))
        (Default|Rotate _asswitch__straightaway)
        (else
          ;;[1 1 1] test to see which resistor and then swap ints
          (if (Utilities|ClassIsChildOf _returnvalue "/Game/Circuit/Light_And_Resistors.Light_And_Resistors_C")
            (bind _aslight_and_resistors (Utilities|Casting|CastToLight_And_Resistors (Variables|Default|GetLeftClick%20Hit%20Actor)))
            (if (Utilities|Enum|Equal(Enum) (Utilities|GetObjectName (Variables|/Game/Circuit/Light_And_Resistors.Light_And_Resistors_C|GetResistor1-GREEN _aslight_and_resistors)) (Utilities|GetObjectName (Variables|Default|GetHit%20Component)))
              (Default|CycleThroughResistor1Power _aslight_and_resistors)
              (elif (Utilities|Enum|Equal(Enum) (Utilities|GetObjectName (Variables|Default|GetHit%20Component)) (Utilities|GetObjectName (Variables|/Game/Circuit/Light_And_Resistors.Light_And_Resistors_C|GetResistor2-RED _aslight_and_resistors)))
                (Default|CycleThroughResistor2Power _aslight_and_resistors)))))))))

(event Input|ActionEvents|InputActionToggleInput
  (params (Key :type Key%20Structure :default "None"))
  (:Pressed
    (Variables|Default|SetLeftClick true))
  (:Released
    (Variables|Default|SetLeftClick false)))

(event Input|AxisEvents|InputAxisMoveForward
  (params (AxisValue :type Float%20%28single-precision%29))
  ;[1 1 1] Movement WASD
  (Pawn|Input|AddMovementInput (Pawn|GetControlledPawn) (Math|Vector|GetForwardVector (Math|Rotator|MakeRotator (.Yaw (Math|Rotator|BreakRotator (Pawn|GetControlRotation :!class /Script/Engine.Controller))) 0.0 0.0)) AxisValue false))

(event Input|AxisEvents|InputAxisMoveRight
  (params (AxisValue :type Float%20%28single-precision%29))
  ;[1 1 1] Movement WASD
  (Pawn|Input|AddMovementInput (Pawn|GetControlledPawn) (Math|Vector|GetRightVector (Math|Rotator|MakeRotator (.Yaw (Math|Rotator|BreakRotator (Pawn|GetControlRotation :!class /Script/Engine.Controller))) 0.0 0.0)) AxisValue false))

(fn ConstructionScript)